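; BP_Key is an interactable key pickup that unlocks a linked Door for the first-person character.
; A sphere overlap registers the key as the character's LastInteractObj and sets CanInteract while the player is in range.
; The Interact event sets HasKey on the Door reference and destroys the key.
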(event `self.Sphere.OnComponentBeginOverlap`
  (params (OverlappedComponent :type "PrimitiveComponent Object Reference") (OtherActor :type "Actor Object Reference") (OtherComp :type "PrimitiveComponent Object Reference") (OtherBodyIndex :type Integer) (bFromSweep :type Boolean) (SweepResult :type "HitResult Structure (by ref)"))
  (bind _asbp_first_person_character (cast `/Game/FirstPerson/Blueprints/BP_FirstPersonCharacter` OtherActor))
  (set `/Game/FirstPerson/Blueprints/BP_FirstPersonCharacter.LastInteractObj` self _asbp_first_person_character)
  (set `self.CanInteract?` true))

(event `self.Sphere.OnComponentEndOverlap`
  (params (OverlappedComponent :type "PrimitiveComponent Object Reference") (OtherActor :type "Actor Object Reference") (OtherComp :type "PrimitiveComponent Object Reference") (OtherBodyIndex :type Integer))
  (cast `/Game/FirstPerson/Blueprints/BP_FirstPersonCharacter` OtherActor)
  (set `self.CanInteract?` false))

(event `/Game/Blueprints/Interface/Interact-Interface.Interact`
  (set `/Game/Blueprints/BP/BP_Interact/BP_Door.HasKey?` true (`self.Door`))
  (`self.K2_DestroyActor`))

(fn `UserConstructionScript`)