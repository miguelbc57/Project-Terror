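; BP_Bomb is an interactable bomb actor that explodes two seconds after Interact is called.
; A Sphere overlap registers it as the first-person character's LastInteractObj and toggles CanInteract, which Interact itself never checks.
; Interact waits, calls DestroyActor, then sets Exploded and plays the explosion sound.
; ExplosionArea only flags TookDamage when the character begins overlapping while Exploded is true, applying no damage itself.
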(event `self.Sphere.OnComponentBeginOverlap`
  (params (OverlappedComponent :type "PrimitiveComponent Object Reference") (OtherActor :type "Actor Object Reference") (OtherComp :type "PrimitiveComponent Object Reference") (OtherBodyIndex :type Integer) (bFromSweep :type Boolean) (SweepResult :type "HitResult Structure (by ref)"))
  (bind _asbp_first_person_character (cast `/Game/FirstPerson/Blueprints/BP_FirstPersonCharacter` OtherActor))
  (set `/Game/FirstPerson/Blueprints/BP_FirstPersonCharacter.LastInteractObj` self _asbp_first_person_character)
  (set `self.CanInteract?` true))

(event `self.Sphere.OnComponentEndOverlap`
  (params (OverlappedComponent :type "PrimitiveComponent Object Reference") (OtherActor :type "Actor Object Reference") (OtherComp :type "PrimitiveComponent Object Reference") (OtherBodyIndex :type Integer))
  (cast `/Game/FirstPerson/Blueprints/BP_FirstPersonCharacter` OtherActor)
  (set `self.CanInteract?` false))

(event `/Game/Blueprints/Interface/Interact-Interface.Interact`
  (`KismetSystemLibrary.Delay` 2.0)
  (`self.K2_DestroyActor` self)
  (set `self.Exploded?` true)
  (`GameplayStatics.PlaySoundAtLocation` "/Game/Sounds/Explosão.Explosão" (`self.K2_GetActorLocation`) (struct) 1.0 1.0 0.0 null null null null))

(event `self.Explosion-Area.OnComponentBeginOverlap`
  (params (OverlappedComponent :type "PrimitiveComponent Object Reference") (OtherActor :type "Actor Object Reference") (OtherComp :type "PrimitiveComponent Object Reference") (OtherBodyIndex :type Integer) (bFromSweep :type Boolean) (SweepResult :type "HitResult Structure (by ref)"))
  (cast `/Game/FirstPerson/Blueprints/BP_FirstPersonCharacter` OtherActor)
  (if (`self.Exploded?`)
    (set `self.TookDamage?` true)))

(fn `UserConstructionScript`)