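; BP_Door is a key-gated door that swings open and closed when interacted with.
; A Box overlap registers it as the first-person character's LastInteractObj and enables interaction until the character leaves.
; Interact uses a FlipFlop to alternate between opening, which requires HasKey, and closing, advancing even when the attempt fails.
; A Timeline drives the mesh's yaw forward or in reverse and sets DoorOpen when finished.
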(event `self.Box.OnComponentBeginOverlap`
  (params (OverlappedComponent :type "PrimitiveComponent Object Reference") (OtherActor :type "Actor Object Reference") (OtherComp :type "PrimitiveComponent Object Reference") (OtherBodyIndex :type Integer) (bFromSweep :type Boolean) (SweepResult :type "HitResult Structure (by ref)"))
  (bind _asbp_first_person_character (cast `/Game/FirstPerson/Blueprints/BP_FirstPersonCharacter` OtherActor))
  (set `/Game/FirstPerson/Blueprints/BP_FirstPersonCharacter.LastInteractObj` self _asbp_first_person_character)
  (set `self.CanInteract?` true))

(event `self.Box.OnComponentEndOverlap`
  (params (OverlappedComponent :type "PrimitiveComponent Object Reference") (OtherActor :type "Actor Object Reference") (OtherComp :type "PrimitiveComponent Object Reference") (OtherBodyIndex :type Integer))
  (cast `/Game/FirstPerson/Blueprints/BP_FirstPersonCharacter` OtherActor)
  (set `self.CanInteract?` false))

(event `/Game/Blueprints/Interact-Interface.Interact`
  (if (`self.CanInteract?`)
    (`/Engine/EditorBlueprintResources/StandardMacros.FlipFlop`
      (:`A`
        (if (`self.HasKey?`)
          (if (not (`self.DoorOpen?`))
            (bind (_direction _rotation_door) (`Timeline|Timeline` :!via `PlayFromStart` :!label _label)
              (:`Update`
                (`SceneComponent.K2_SetRelativeRotation` (`self.StaticMesh`) (`KismetMathLibrary.MakeRotator` 0.0 0.0 _rotation_door) false false))
              (:`Finished`
                (set `self.DoorOpen?` (> _rotation_door 0.0)))))))
      (:`B`
        (if (`self.DoorOpen?`)
          (goto _label :!via `ReverseFromEnd`))))))

(fn `UserConstructionScript`)